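; BP_Grid is an actor that builds a centered tile grid in the Y-Z plane as instances of one InstancedStaticMesh.
; The construction script calls SpawnGrid with the grid's settings, which stores them, clears old instances and adds one scaled, rotated instance per tile.
; The shape enum's name is the row lookup into DT_GridShapeData, supplying the flat mesh, border material and mesh size used for scaling.
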(event EventBeginPlay)

(event Collision|EventActorBeginOverlap
  (params (OtherActor :type Actor%20Object%20Reference)))

(event EventTick
  (params (DeltaSeconds :type Float%20%28single-precision%29)))

(fn ConstructionScript
  (CallFunction|SpawnGrid (Variables|Default|GetGridCenterLocation) (Variables|Default|GetGridTileSize) (Variables|Default|GetGridTileCount) (Variables|Default|GetGridShape) (Variables|Default|GetGridRotation)))

(fn SpawnGrid
  (params (CenterLocation :type Vector) (TileSize :type Vector) (TileCount :type Vector%202D%20Structure) (Shape :type E_GridShape%20Enum :default "NewEnumerator0") (Rotation :type Rotator))
  (bind _shapedata (CallFunction|GetCurrentShapeData))
  (bind _instancedstaticmesh (Variables|Default|GetInstancedStaticMesh))
  (bind (_meshsize _mesh _meshmaterial _flatmesh _flatbordermaterial) (Utilities|Struct|BreakS_GridShapeData _shapedata))
  (Variables|Default|SetGridCenterLocation CenterLocation)
  (Variables|Default|SetGridTileSize TileSize)
  (Variables|Default|SetGridTileCount TileCount)
  (Variables|Default|SetGridShape Shape)
  (Variables|Default|SetGridRotation Rotation)
  (CallFunction|DestroyGrid)
  (Components|StaticMesh|SetStaticMesh _instancedstaticmesh _flatmesh)
  (Rendering|Material|SetMaterial _instancedstaticmesh 0 _flatbordermaterial)
  (Variables|Default|SetGridBottomLeftCornerLocation (- (Variables|Default|GetGridCenterLocation) (Math|Vector|MakeVector 0.0 (.y (* (/ (Variables|Default|GetGridTileCount) 2.0) (Math|Vector2D|MakeVector2D (.z (Variables|Default|GetGridTileSize)) (.y (Variables|Default|GetGridTileSize))))) (.x (* (/ (Variables|Default|GetGridTileCount) 2.0) (Math|Vector2D|MakeVector2D (.z (Variables|Default|GetGridTileSize)) (.y (Variables|Default|GetGridTileSize))))))))
  (for _index (range 0 (- (Math|Float|Round (.x (Variables|Default|GetGridTileCount))) 1))
    (LocalVariables|SetX%28Z%29 _index)
    (for _index_2 (range 0 (- (Math|Float|Round (.y (Variables|Default|GetGridTileCount))) 1))
      (LocalVariables|SetY _index_2)
      (LocalVariables|SetTileTransform (Math|Transform|MakeTransform (+ (Variables|Default|GetGridBottomLeftCornerLocation) (* (Variables|Default|GetGridTileSize) (Math|Vector|MakeVector 0.0 (Math|Conversions|ToFloat(Integer) (LocalVariables|GetY)) (Math|Conversions|ToFloat(Integer) (LocalVariables|GetX%28Z%29))))) (Variables|Default|GetGridRotation) (/ (Variables|Default|GetGridTileSize) (.MeshSize (Utilities|Struct|BreakS_GridShapeData (CallFunction|GetCurrentShapeData))))))
      (Components|InstancedStaticMesh|AddInstance (Variables|Default|GetInstancedStaticMesh) (LocalVariables|GetTileTransform)))))

(fn GetCurrentShapeData
  (bind _gridshape (Variables|Default|GetGridShape))
  (bind _returnvalue (Utilities|String|EnumtoString _gridshape))
  (bind _returnvalue_2 (Utilities|GetDataTableRow "/Game/Blueprint/Core/Grid/Gridshape/DT_GridShapeData.DT_GridShapeData" (Utilities|String|StringToName _returnvalue))
    (:then
      (return _returnvalue_2))
    (:RowNotFound
      (Development|PrintString (Utilities|String|Append "Error - Not Found -" _returnvalue) true true "(R=1.000000,G=0.000000,B=0.000000,A=1.000000)" 1.0))))

(fn DestroyGrid
  (Components|InstancedStaticMesh|ClearInstances (Variables|Default|GetInstancedStaticMesh)))