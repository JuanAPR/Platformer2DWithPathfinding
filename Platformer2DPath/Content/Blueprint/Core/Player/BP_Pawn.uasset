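; BP_Pawn is a player pawn that pans in a vertical plane and zooms through its spring arm.
; Forward and right axis inputs shift a desired location on Z and Y within clamped bounds, and zoom input sets a clamped arm length.
; Tick also adds normalized up/right input to that location, unclamped and unscaled by delta time, then eases actor position and arm length toward their targets using interpolation.
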(event EventTick
  (params (DeltaSeconds :type Float%20%28single-precision%29))
  (bind _springarm (Variables|Default|GetSpringArm))
  (Variables|Default|SetLocation_Desired (+ (Variables|Default|GetLocation_Desired) (* (Math|Vector|Normalize (+ (* (Transformation|GetActorUpVector) (Input|AxisValues|GetInputAxisForward)) (* (Transformation|GetActorRightVector) (Input|AxisValues|GetInputAxisRight)))) 2e+01)))
  (Variables|/Script/Engine.SpringArmComponent|SetTargetArmLength _springarm (Math|Interpolation|FInterpTo (Variables|/Script/Engine.SpringArmComponent|GetTargetArmLength _springarm) (Variables|Default|GetZoom_Desired) (Utilities|Time|GetWorldDeltaSeconds) 2.0))
  (Transformation|SetActorLocation (Math|Interpolation|VInterpTo (Transformation|GetActorLocation) (Variables|Default|GetLocation_Desired) (Utilities|Time|GetWorldDeltaSeconds) 5.0) false false))

(event EventBeginPlay
  (Variables|Default|SetLocation_Desired (Transformation|GetActorLocation))
  (Variables|Default|SetZoom_Desired (Variables|/Script/Engine.SpringArmComponent|GetTargetArmLength (Variables|Default|GetSpringArm))))

(event Input|AxisEvents|InputAxisInputAxisZoom
  (params (AxisValue :type Float%20%28single-precision%29))
  (Variables|Default|SetZoom_Desired (Math|Float|Clamp(Float) (+ (Variables|Default|GetZoom_Desired) (* AxisValue 5e+01)) 5e+02 5e+03)))

(event Input|AxisEvents|InputAxisInputAxisForward
  (params (AxisValue :type Float%20%28single-precision%29))
  (Variables|Default|SetLocation_Desired (Math|Vector|MakeVector (.x (+ (Variables|Default|GetLocation_Desired) (Math|Vector|MakeVector 0.0 0.0 (* AxisValue 2e+01)))) (.y (+ (Variables|Default|GetLocation_Desired) (Math|Vector|MakeVector 0.0 0.0 (* AxisValue 2e+01)))) (Math|Float|Clamp(Float) (.z (+ (Variables|Default|GetLocation_Desired) (Math|Vector|MakeVector 0.0 0.0 (* AxisValue 2e+01)))) 0.0 1e+04))))

(event Input|AxisEvents|InputAxisInputAxisRight
  (params (AxisValue :type Float%20%28single-precision%29))
  (Variables|Default|SetLocation_Desired (Math|Vector|MakeVector (.x (+ (Variables|Default|GetLocation_Desired) (Math|Vector|MakeVector 0.0 (* AxisValue 2e+01) 0.0))) (Math|Float|Clamp(Float) (.y (+ (Variables|Default|GetLocation_Desired) (Math|Vector|MakeVector 0.0 (* AxisValue 2e+01) 0.0))) -2e+02 1e+04) (.z (+ (Variables|Default|GetLocation_Desired) (Math|Vector|MakeVector 0.0 (* AxisValue 2e+01) 0.0))))))

(fn ConstructionScript)